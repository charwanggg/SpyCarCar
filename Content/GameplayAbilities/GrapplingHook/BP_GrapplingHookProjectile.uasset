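; BP_GrapplingHookProjectile is the projectile actor for the grappling hook ability.
; On a collision hit it records the hit actor, zeroes its projectile movement velocity and flags itself as connected.
; Once connected, Tick accumulates time alive and destroys the actor when that exceeds its lifetime, so time in flight does not count.
; A Cable component is present but unused in the graph.
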(event OnComponentHit(Collision)
  (params (HitComponent :type Primitive%20Component%20Object%20Reference) (OtherActor :type Actor%20Object%20Reference) (OtherComp :type Primitive%20Component%20Object%20Reference) (NormalImpulse :type Vector :default "0, 0, 0") (Hit :type Hit%20Result%20Structure%20%28by%20ref%29))
  (Variables|Default|SetHitActor OtherActor)
  (Game|Components|ProjectileMovement|SetVelocityinLocalSpace (Variables|Default|GetProjectileMovement) "0, 0, 0")
  (Variables|Default|SetIsConnected true))

(event EventBeginPlay
  (Actor|GetActorOfClass 0))

(event Collision|EventActorBeginOverlap
  (params (OtherActor :type Actor%20Object%20Reference)))

(event EventTick
  (params (DeltaSeconds :type Float%20%28single-precision%29))
  (if (Variables|Default|GetIsConnected)
    (bind _output_get (Variables|Default|SetTime%20Alive (+ DeltaSeconds (Variables|Default|GetTime%20Alive))))
    (Math|Float|CompareFloat _output_get (Variables|Default|GetLifetime)
      (:>
        (Actor|DestroyActor)))))

(fn ConstructionScript)