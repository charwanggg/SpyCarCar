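; BP_Flamethrower is a timed flamethrower effect actor that follows its Gun and deals area damage until its Duration expires.
; Each Tick it snaps to the Gun's transform and spawns a BP_HitBox ahead of the muzzle, passing radius, damage and attacker.
; Sphere overlaps still track BP_HP components in Targets, excluding BP_SpyCar, but the direct damage loop that reads them is disconnected.
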(event OnComponentBeginOverlap(Sphere)
  (params (OverlappedComponent :type Primitive%20Component%20Object%20Reference) (OtherActor :type Actor%20Object%20Reference) (OtherComp :type Primitive%20Component%20Object%20Reference) (OtherBodyIndex :type Integer) (bFromSweep :type Boolean) (SweepResult :type Hit%20Result%20Structure%20%28by%20ref%29))
  (Utilities|Casting|CastToBP_SpyCar OtherActor
    (:CastFailed
      (Utilities|Array|AddUnique (Variables|Default|GetTargets) (Actor|GetComponentbyClass OtherActor "/Game/BluePrints/BP_HP.BP_HP_C")))))

(event OnComponentEndOverlap(Sphere)
  (params (OverlappedComponent :type Primitive%20Component%20Object%20Reference) (OtherActor :type Actor%20Object%20Reference) (OtherComp :type Primitive%20Component%20Object%20Reference) (OtherBodyIndex :type Integer))
  (Utilities|Casting|CastToBP_SpyCar OtherActor
    (:CastFailed
      (Utilities|Array|RemoveItem (Variables|Default|GetTargets) (Actor|GetComponentbyClass OtherActor "/Game/BluePrints/BP_HP.BP_HP_C")))))

(event EventBeginPlay
  (Variables|Default|SetdoneTime (+ (Variables|Default|GetDuration) (Utilities|Time|GetGameTimeinSeconds))))

(event Collision|EventActorBeginOverlap
  (params (OtherActor :type Actor%20Object%20Reference)))

(event EventTick
  (params (DeltaSeconds :type Float%20%28single-precision%29))
  (bind _gun (Variables|Default|GetGun))
  (bind _returnvalue (Transformation|GetActorTransform _gun))
  (bind (_location _rotation) (Math|Transform|BreakTransform _returnvalue))
  (if (> (Utilities|Time|GetGameTimeinSeconds) (Variables|Default|GetdoneTime))
    (Actor|DestroyActor)
    (else
      (Transformation|SetActorTransform (Math|Transform|MakeTransform _location _rotation))
      (Game|SpawnActorfromClass "/Game/BluePrints/BP_HitBox.BP_HitBox_C" (Math|Transform|MakeTransform (+ _location (* (Math|Vector|GetForwardVector (Variables|/Game/BluePrints/BP_CarGun.BP_CarGun_C|GetDefaultSceneRoot _gun)) 2e+02))) "Undefined" "MultiplyWithRoot" 0 0.25 4e+02 50 0.0 (Variables|Default|GetAttacker) 0))))

(fn ConstructionScript)