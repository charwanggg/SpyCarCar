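; BP_RockBallExplode1 is a short-lived destruction effect for the Rockball ability that breaks a rock into tumbling pieces.
; On BeginPlay it crumbles the root cluster of its Geometry Collection, applies angular velocity to that item and plays the StartPlayInEditor sound at world origin rather than the actor's location.
; Tick accumulates time alive and destroys the actor after ten seconds.
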(event EventBeginPlay
  (bind _geometrycollection1 (Variables|Default|GetGeometryCollection1))
  (Audio|PlaySoundatLocation "/Engine/EditorSounds/GamePreview/StartPlayInEditor.StartPlayInEditor" "0, 0, 0" "0, 0, 0" 1.0 1.0 0.0 0 0 0 0)
  (Class|GeometryCollectionComponent|CrumbleCluster _geometrycollection1)
  (Class|GeometryCollectionComponent|ApplyAngularVelocity _geometrycollection1 0 (Math|Vector|MakeVector 2e+01 2e+01 2e+01)))

(event Collision|EventActorBeginOverlap
  (params (OtherActor :type Actor%20Object%20Reference)))

(event EventTick
  (params (DeltaSeconds :type Float%20%28single-precision%29))
  (Variables|Default|SetTimeAlive (+ DeltaSeconds (Variables|Default|GetTimeAlive)))
  (if (> (Variables|Default|GetTimeAlive) 1e+01)
    (Actor|DestroyActor)))

(fn ConstructionScript)