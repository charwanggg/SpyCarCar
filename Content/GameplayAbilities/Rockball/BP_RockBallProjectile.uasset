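; BP_RockBallProjectile is a tumbling rock projectile that stops on impact and bursts after a delay.
; On BeginPlay it randomizes the Rock17 mesh's rotation and spin, and caches the gun out point and spy car actors.
; A collision hit zeroes velocity and spin and starts a lifetime timer on Tick.
; When the timer expires, it spawns BP_RockBallExplode with the rock's location and rotation, then destroys itself.
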(event OnComponentHit(Collision)
  (params (HitComponent :type Primitive%20Component%20Object%20Reference) (OtherActor :type Actor%20Object%20Reference) (OtherComp :type Primitive%20Component%20Object%20Reference) (NormalImpulse :type Vector :default "0, 0, 0") (Hit :type Hit%20Result%20Structure%20%28by%20ref%29))
  (Variables|Default|SetHitActor OtherActor)
  (Game|Components|ProjectileMovement|SetVelocityinLocalSpace (Variables|Default|GetProjectileMovement) "0, 0, 0")
  (Variables|Default|SetRotationRandom "0, 0, 0")
  (Variables|Default|SetOnGround true))

(event EventBeginPlay
  (bind _returnvalue (Math|Random|RandomRotator false))
  (bind _returnvalue_2 (Actor|GetActorOfClass "/Game/BluePrints/BP_GunOutPoint.BP_GunOutPoint_C"))
  (Variables|Default|SetSpyCar _returnvalue_2)
  (bind _returnvalue_3 (Actor|GetActorOfClass "/Game/BluePrints/BP_SpyCar.BP_SpyCar_C"))
  (Variables|Default|SetSpyCarObj _returnvalue_3)
  (Transformation|SetWorldRotation (Variables|Default|Getrock_17) _returnvalue false false)
  (Variables|Default|SetRotationRandom _returnvalue))

(event Collision|EventActorBeginOverlap
  (params (OtherActor :type Actor%20Object%20Reference)))

(event EventTick
  (params (DeltaSeconds :type Float%20%28single-precision%29))
  (Transformation|AddLocalRotation (Variables|Default|Getrock_17) (* (Variables|Default|GetRotationRandom) DeltaSeconds) false false)
  (if (Variables|Default|GetOnGround)
    (Variables|Default|SetTimeAlive (+ DeltaSeconds (Variables|Default|GetTimeAlive)))
    (if (> (Variables|Default|GetTimeAlive) (Variables|Default|GetLifetime))
      (Game|SpawnActorfromClass "/Game/GameplayAbilities/Rockball/BP_RockBallExplode.BP_RockBallExplode_C" (Math|Transform|MakeTransform (.location (Transformation|GetActorTransform)) (Variables|/Script/Engine.SceneComponent|GetRelativeRotation (Variables|Default|Getrock_17)) "1.000000,1.000000,1.000000") "Undefined" "MultiplyWithRoot" 0 0)
      (Actor|DestroyActor))))

(fn ConstructionScript)