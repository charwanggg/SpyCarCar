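; BP_CarGunControl is the spy car's gun actor, which aims with the camera and hosts the weapon abilities.
; On BeginPlay it finds BP_SpyCar and grants Fireball, Grappling Hook and Lightning through its Gameplay Ability System component.
; Each tick it copies the car camera pivot's relative rotation as its actor rotation.
; Separate events activate each ability by gameplay tag.
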(event Custom|FireballAbility
  (Abilities|TryActivateAbilitiesbyTag (Variables|Default|GetAbilitySystem) (Variables|Default|GetFireball%20Tag) true))

(event Custom|GrapplingHookAbility
  (Abilities|TryActivateAbilitiesbyTag (Variables|Default|GetAbilitySystem) (Variables|Default|GetGrapplingHook%20Tag) true))

(event Custom|LightningAbility
  (Abilities|TryActivateAbilitiesbyTag (Variables|Default|GetAbilitySystem) (Variables|Default|GetLightning%20Tag) true))

(event EventBeginPlay
  (bind _abilitysystem (Variables|Default|GetAbilitySystem))
  (bind _returnvalue (Actor|GetActorOfClass "/Game/BluePrints/BP_SpyCar.BP_SpyCar_C"))
  (Variables|Default|SetSpycar _returnvalue)
  (GameplayAbilities|GiveAbility _abilitysystem "/Game/GameplayAbilities/Fireball/GA_Fireball.GA_Fireball_C" 0 -1)
  (GameplayAbilities|GiveAbility _abilitysystem "/Game/GameplayAbilities/GrapplingHook/GA_GrapplingHook.GA_GrapplingHook_C" 0 -1)
  (GameplayAbilities|GiveAbility _abilitysystem "/Game/GameplayAbilities/Lightning/GA_Lightning.GA_Lightning_C" 0 -1))

(event Collision|EventActorBeginOverlap
  (params (OtherActor :type Actor%20Object%20Reference)))

(event EventTick
  (params (DeltaSeconds :type Float%20%28single-precision%29))
  (Transformation|SetActorRotation (Variables|/Script/Engine.SceneComponent|GetRelativeRotation (Variables|/Game/BluePrints/BP_SpyCar.BP_SpyCar_C|GetCameraPivot (Variables|Default|GetSpycar)))))

(fn ConstructionScript)