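; Player-driven spy car pawn that can climb walls, using a physics sphere for movement and a cube that follows it for orientation.
; Enhanced Input pushes the sphere along the cube's forward vector, yaws the cube and sets a brake flag nothing here reads.
; Each tick caps speed and traces forward-down for surface normals; while throttle is held, a state enum drives alignment and grip force, otherwise the car can ease upright.
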(event Input|EnhancedActionEvents|EnhancedInputActionIA_MoveForward
  (params (ActionValue :type Float%20%28double-precision%29) (ElapsedSeconds :type Float%20%28double-precision%29) (TriggeredSeconds :type Float%20%28double-precision%29) (InputAction :type Input%20Action%20Object%20Reference :default "/Game/BluePrints/IA_MoveForward.IA_MoveForward"))
  (:Triggered
    (Physics|AddForce (Variables|Default|GetSphere) (* (* ActionValue (Variables|Default|GetThrottleForce)) (Math|Vector|GetForwardVector (Variables|Default|GetCube))) "None" false)
    (Variables|Default|SetIsGripped true))
  (:Completed
    (Variables|Default|SetIsGripped false)))

(event Input|EnhancedActionEvents|EnhancedInputActionIA_Steering
  (params (ActionValue :type Float%20%28double-precision%29) (ElapsedSeconds :type Float%20%28double-precision%29) (TriggeredSeconds :type Float%20%28double-precision%29) (InputAction :type Input%20Action%20Object%20Reference :default "/Game/BluePrints/IA_Steering.IA_Steering"))
  (:Triggered
    (Variables|Default|SetTurnInput ActionValue :!label _label))
  (:Ongoing
    (goto _label))
  (:Completed
    (Variables|Default|SetTurnInput 0.0)))

(event Input|EnhancedActionEvents|EnhancedInputActionIA_Brake
  (params (ActionValue :type Boolean) (ElapsedSeconds :type Float%20%28double-precision%29) (TriggeredSeconds :type Float%20%28double-precision%29) (InputAction :type Input%20Action%20Object%20Reference :default "/Game/BluePrints/IA_Brake.IA_Brake"))
  (:Triggered
    (Variables|Default|SetisBraking true))
  (:Completed
    (Variables|Default|SetisBraking false)))

(event EventBeginPlay
  (bind _asplayer_controller (Utilities|Casting|CastToPlayerController (Pawn|GetController)))
  (Utilities|IsValid (PlayerController|LocalPlayerSubsystems|GetEnhancedInputLocalPlayerSubsystem _asplayer_controller)
    (:Is%20Valid
      (Input|AddMappingContext (PlayerController|LocalPlayerSubsystems|GetEnhancedInputLocalPlayerSubsystem _asplayer_controller) "/Game/BluePrints/IMC_SpyCar.IMC_SpyCar" 0 "(bIgnoreAllPressedKeysUntilRelease=True,bForceImmediately=False,bNotifyUserSettings=False)"))))

(event Collision|EventActorBeginOverlap
  (params (OtherActor :type Actor%20Object%20Reference)))

(event EventTick
  (params (DeltaSeconds :type Float%20%28single-precision%29))
  (CallFunction|Steer)
  (CallFunction|HandleWallClimb)
  (CallFunction|CapsPeed)
  (CallFunction|RaycastCheckWall)
  (Transformation|SetWorldLocation (Variables|Default|GetCube) (.Location (Math|Transform|BreakTransform (Transformation|GetWorldTransform (Variables|Default|GetSphere)))) false false))

(fn ConstructionScript)

(fn CapsPeed
  (bind _sphere (Variables|Default|GetSphere))
  (bind _maxspeed (Variables|Default|GetMaxSpeed))
  (bind _returnvalue (Physics|GetPhysicsLinearVelocity _sphere "None"))
  (if (> (Math|Vector|VectorLength _returnvalue) _maxspeed)
    (Physics|SetPhysicsLinearVelocity _sphere (* _maxspeed (Math|Vector|Normalize _returnvalue)) false "None")
    (Development|PrintString "Capping")))

(fn Steer
  (Transformation|AddLocalRotation (Variables|Default|GetCube) (Math|Rotator|MakeRotator 0.0 0.0 (* (* (Variables|Default|GetTurnSpeed) (Utilities|Time|GetWorldDeltaSeconds)) (Variables|Default|GetTurnInput))) false false))

(fn HandleWallClimb
  (bind _cube (Variables|Default|GetCube))
  (if (Variables|Default|GetIsGripped)
    (if (== (Variables|Default|GetState) 1)
      (Development|PrintString "OnWall")
      (Physics|AddForce (Variables|Default|GetSphere) (* (Variables|Default|GetCurrentUp) (* (Variables|Default|GetWallGripStrength) -1.0)) "None" false)
      (CallFunction|AlignCar)
      (elif (== (Variables|Default|GetState) 2)
        (bind _returnvalue (CallFunction|AlignCar))
        (if _returnvalue
          (Variables|Default|SetState "NewEnumerator1"))))
    (elif (!= (Variables|Default|GetState) 0)
      (bind _output_get (Variables|Default|SetCurrentUp "0.000000,0.000000,1.000000"))
      (Transformation|SetWorldRotation _cube (Math|Interpolation|RInterpTo (Transformation|GetWorldRotation _cube) (Math|Rotator|MakeRotfromZX _output_get (Math|Vector|GetForwardVector _cube)) (Utilities|Time|GetWorldDeltaSeconds) 1e+01) false false))))

(fn AlignCar
  (bind _cube (Variables|Default|GetCube))
  (bind _returnvalue (Transformation|GetWorldRotation _cube))
  (Transformation|SetWorldRotation _cube (Math|Interpolation|RInterpTo _returnvalue (Math|Rotator|MakeRotfromZY (Variables|Default|GetCurrentUp) (Math|Vector|GetRightVector _cube)) (Utilities|Time|GetWorldDeltaSeconds) 1e+01) false false)
  (return (Utilities|Operators|EqualEqual :B _returnvalue :ErrorTolerance 0.01)))

(fn RaycastCheckWall
  (bind _cube (Variables|Default|GetCube))
  (bind _returnvalue (Transformation|GetWorldLocation _cube))
  (bind _returnvalue_2 (Math|Vector|GetForwardVector _cube))
  (bind _returnvalue_3 (* _returnvalue_2 5e+01))
  (bind _returnvalue_4 (+ _returnvalue_3 _returnvalue))
  (bind (_outhit _returnvalue_5) (Collision|LineTraceByChannel _returnvalue_4 (+ _returnvalue_4 (* (- _returnvalue_2 (Math|Vector|GetUpVector _cube)) (Variables|Default|GetLineTraceLength))) "TraceTypeQuery1" false 0 "ForOneFrame"))
  (if _returnvalue_5
    (Variables|Default|SetCurrentUp (.Normal (Collision|BreakHitResult _outhit)))
    (if (Variables|Default|GetIsGripped)
      (Variables|Default|SetState "NewEnumerator2"))))