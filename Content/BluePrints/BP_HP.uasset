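; BP_HP is a reusable health Blueprint that tracks current and maximum HP.
; Initialize sets the maximum and fills current HP to it.
; TakeDamage subtracts damage without clamping and fires a damage dispatcher, then a death dispatcher whenever HP is at or below zero.
; It has no guard against repeated death calls, and its Tick and BeginPlay are empty.
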(event Custom|TakeDamage
  (params (Damage :type Integer))
  (Variables|Default|SetHP (- (Variables|Default|GetHP) Damage))
  (Default|CallTakeDamage)
  (if (<= (Variables|Default|GetHP) 0)
    (Default|CallDeath)))

(event Custom|Initialize
  (params (Max%20Health :type Integer))
  (bind _output_get (Variables|Default|SetMax%20HP Max%20Health))
  (Variables|Default|SetHP _output_get))

(event EventBeginPlay)

(event EventTick
  (params (DeltaSeconds :type Float%20%28single-precision%29)))