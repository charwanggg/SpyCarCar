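; BP_Turret is a stationary-style enemy turret that fires at the player's spy car when it comes within range.
; A detection sphere sized by Range starts and stops the shooting component as a BP_SpyCar enters or leaves.
; While shooting, Tick aims the component's fire direction from the arrow muzzle toward player pawn 0.
; An HP component destroys the turret on death.
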(event OnComponentBeginOverlap(Sphere)
  (params (OverlappedComponent :type Primitive%20Component%20Object%20Reference) (OtherActor :type Actor%20Object%20Reference) (OtherComp :type Primitive%20Component%20Object%20Reference) (OtherBodyIndex :type Integer) (bFromSweep :type Boolean) (SweepResult :type Hit%20Result%20Structure%20%28by%20ref%29))
  (Utilities|Casting|CastToBP_SpyCar OtherActor)
  (Default|Shoot (Variables|Default|GetBP_Shooting))
  (Development|PrintString "begin shooting"))

(event OnComponentEndOverlap(Sphere)
  (params (OverlappedComponent :type Primitive%20Component%20Object%20Reference) (OtherActor :type Actor%20Object%20Reference) (OtherComp :type Primitive%20Component%20Object%20Reference) (OtherBodyIndex :type Integer))
  (Utilities|Casting|CastToBP_SpyCar OtherActor)
  (Default|StopShooting (Variables|Default|GetBP_Shooting)))

(event Custom|Die
  (Actor|DestroyActor))

(event EventBeginPlay
  (bind _bp_hp (Variables|Default|GetBP_HP))
  (Components|Sphere|SetSphereRadius (Variables|Default|GetSphere) (Variables|Default|GetRange) true)
  (Default|Initialize (Variables|Default|GetBP_Shooting) 5 (Transformation|GetWorldLocation (Variables|Default|GetArrow)) 40)
  (Default|Initialize _bp_hp 100)
  (EventDispatchers|BindEventtoDeath _bp_hp (delegate Custom|Die)))

(event Collision|EventActorBeginOverlap
  (params (OtherActor :type Actor%20Object%20Reference)))

(event EventTick
  (params (DeltaSeconds :type Float%20%28single-precision%29))
  (bind _bp_shooting (Variables|Default|GetBP_Shooting))
  (if (Variables|/Game/BluePrints/BP_Shooting.BP_Shooting_C|GetIsShooting _bp_shooting)
    (Variables|/Game/BluePrints/BP_Shooting.BP_Shooting_C|SetDirection _bp_shooting (- (Transformation|GetActorLocation (Game|Player|GetPlayerPawn 0)) (Transformation|GetWorldLocation (Variables|Default|GetArrow))))))

(fn ConstructionScript)