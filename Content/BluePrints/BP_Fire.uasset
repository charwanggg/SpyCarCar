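; BP_Fire is a damage-over-time hazard actor that hurts spy cars standing inside its Box volume.
; Box overlap begin and end events add or remove each BP_SpyCar's BPHP health component in a Targets array, with a leftover debug print on entry.
; Tick compares game time against NextTick to apply DamagePerTick to every target once per TickInterval.
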(event OnComponentBeginOverlap(Box)
  (params (OverlappedComponent :type Primitive%20Component%20Object%20Reference) (OtherActor :type Actor%20Object%20Reference) (OtherComp :type Primitive%20Component%20Object%20Reference) (OtherBodyIndex :type Integer) (bFromSweep :type Boolean) (SweepResult :type Hit%20Result%20Structure%20%28by%20ref%29))
  (Development|PrintString "Hello")
  (bind _asbp_spy_car (Utilities|Casting|CastToBP_SpyCar OtherActor))
  (Utilities|Array|AddUnique (Variables|Default|GetTargets) (Variables|/Game/BluePrints/BP_SpyCar.BP_SpyCar_C|GetBP_HP _asbp_spy_car)))

(event OnComponentEndOverlap(Box)
  (params (OverlappedComponent :type Primitive%20Component%20Object%20Reference) (OtherActor :type Actor%20Object%20Reference) (OtherComp :type Primitive%20Component%20Object%20Reference) (OtherBodyIndex :type Integer))
  (bind _asbp_spy_car (Utilities|Casting|CastToBP_SpyCar OtherActor))
  (Utilities|Array|RemoveItem (Variables|Default|GetTargets) (Variables|/Game/BluePrints/BP_SpyCar.BP_SpyCar_C|GetBP_HP _asbp_spy_car)))

(event EventBeginPlay)

(event Collision|EventActorBeginOverlap
  (params (OtherActor :type Actor%20Object%20Reference)))

(event EventTick
  (params (DeltaSeconds :type Float%20%28single-precision%29))
  (if (> (Utilities|Time|GetGameTimeinSeconds) (Variables|Default|GetNext%20Tick))
    (for _array_element (Variables|Default|GetTargets)
      (Default|TakeDamage _array_element (Variables|Default|GetDamagePerTick)))
    (Variables|Default|SetNext%20Tick (+ (Utilities|Time|GetGameTimeinSeconds) (Variables|Default|GetTick%20Interval)))))

(fn ConstructionScript)