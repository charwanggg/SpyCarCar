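; BP_Bullet is a projectile actor that damages what it hits.
; When its Sphere component begins an overlap, it ignores its owner and looks for a BP_HP component on the other valid actor.
; If one exists, it passes BulletDamage to TakeDamage; either way, the bullet then destroys itself.
; An unconnected leftover branch with a debug print never runs, and the graph contains no movement logic.
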(event OnComponentBeginOverlap(Sphere)
  (params (OverlappedComponent :type Primitive%20Component%20Object%20Reference) (OtherActor :type Actor%20Object%20Reference) (OtherComp :type Primitive%20Component%20Object%20Reference) (OtherBodyIndex :type Integer) (bFromSweep :type Boolean) (SweepResult :type Hit%20Result%20Structure%20%28by%20ref%29))
  (bind _returnvalue (Actor|GetComponentbyClass OtherActor "/Game/BluePrints/BP_HP.BP_HP_C"))
  (Utilities|IsValid OtherActor
    (:Is%20Valid
      (if (not (== OtherActor (Components|GetOwner)))
        (Utilities|IsValid _returnvalue
          (:Is%20Valid
            (Default|TakeDamage _returnvalue (Variables|Default|GetBulletDamage))
            (Actor|DestroyActor))
          (:Is%20Not%20Valid
            (Actor|DestroyActor)))))))

(event EventBeginPlay)

(event Collision|EventActorBeginOverlap
  (params (OtherActor :type Actor%20Object%20Reference)))

(event EventTick
  (params (DeltaSeconds :type Float%20%28single-precision%29)))

(fn ConstructionScript)