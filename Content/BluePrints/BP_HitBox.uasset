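; BP_HitBox is a short-lived spherical hit volume that damages and knocks back actors it overlaps, ignoring its Attacker.
; On BeginPlay it sizes the sphere to Radius and sets a timer to destroy itself after Lifetime.
; Overlapped actors with a BP_HP component take Damage, and Characters among them are launched away from the hitbox center by Knockback plus a fixed upward boost.
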(event OnComponentBeginOverlap(Sphere)
  (params (OverlappedComponent :type Primitive%20Component%20Object%20Reference) (OtherActor :type Actor%20Object%20Reference) (OtherComp :type Primitive%20Component%20Object%20Reference) (OtherBodyIndex :type Integer) (bFromSweep :type Boolean) (SweepResult :type Hit%20Result%20Structure%20%28by%20ref%29))
  (bind _returnvalue (Actor|GetComponentbyClass OtherActor "/Game/BluePrints/BP_HP.BP_HP_C"))
  (bind _returnvalue_2 (Transformation|GetActorLocation OtherActor))
  (bind _returnvalue_3 (Transformation|GetActorLocation))
  (bind _knockback (Variables|Default|GetKnockback))
  (bind _returnvalue_4 (- _returnvalue_2 _returnvalue_3))
  (bind _returnvalue_5 (Math|Vector|Normalize _returnvalue_4))
  (bind (_x _y _z) (Math|Vector|BreakVector _returnvalue_5))
  (Utilities|IsValid OtherActor
    (:Is%20Valid
      (if (!= OtherActor (Variables|Default|GetAttacker))
        (Utilities|IsValid _returnvalue
          (:Is%20Valid
            (Default|TakeDamage _returnvalue (Variables|Default|GetDamage))
            (bind _ascharacter (Utilities|Casting|CastToCharacter OtherActor))
            (Character|LaunchCharacter _ascharacter (Math|Vector|MakeVector (* _x _knockback) (* _y _knockback) (+ (* _z _knockback) 2e+02)) false false)))))))

(event Custom|DestroySelf
  (Actor|DestroyActor))

(event EventBeginPlay
  (Components|Sphere|SetSphereRadius (Variables|Default|GetSphere) (Variables|Default|GetRadius) true)
  (Utilities|Time|SetTimerbyFunctionName 0 "DestroySelf" (Variables|Default|GetLifetime)))

(event EventTick
  (params (DeltaSeconds :type Float%20%28single-precision%29)))

(fn ConstructionScript)