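; BP_Shooting is a reusable shooting Blueprint that handles automatic fire, ammo and reloading for its owner.
; Initialize sets magazine size, muzzle location and damage, while Shoot and StopShooting toggle the firing flag.
; Tick compares game time against stored timestamps to spawn BP_Bullet along Direction at a fixed interval, passing damage and owner.
; Firing on an empty magazine starts a timed reload that refills it.
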(event Custom|Initialize
  (params (MaxBullets :type Integer) (Muzzle :type Vector) (Damage :type Integer))
  (bind _output_get (Variables|Default|SetMaxBullets MaxBullets))
  (Variables|Default|SetCurrBullets _output_get)
  (Variables|Default|SetMuzzle Muzzle)
  (Variables|Default|SetDamage Damage))

(event Custom|Shoot
  (Variables|Default|SetIsShooting true))

(event Custom|Stop%20Shooting
  (Variables|Default|SetIsShooting false))

(event EventBeginPlay)

(event EventTick
  (params (DeltaSeconds :type Float%20%28single-precision%29))
  (bind _returnvalue (Utilities|Time|GetGameTimeinSeconds))
  (bind _returnvalue_2 (Utilities|Time|GetGameTimeinSeconds))
  (if (Variables|Default|GetIsReloading)
    (if (> _returnvalue (Variables|Default|GetReloadDoneTime))
      (Variables|Default|SetIsReloading false)
      (Variables|Default|SetCurrBullets (Variables|Default|GetMaxBullets)))
    (elif (Variables|Default|GetIsShooting)
      (if (> (Variables|Default|GetCurrBullets) 0)
        (if (> _returnvalue (Variables|Default|GetNextBulletTime))
          (Variables|Default|SetNextBulletTime (+ _returnvalue_2 (Variables|Default|GetBulletInterval)))
          (Game|SpawnActorfromClass "/Game/BluePrints/BP_Bullet.BP_Bullet_C" (Math|Transform|MakeTransform (Variables|Default|GetMuzzle) (Math|Rotator|MakeRotfromX (Variables|Default|GetDirection))) "AlwaysSpawn" "MultiplyWithRoot" (Components|GetOwner) (Variables|Default|GetDamage) 0)
          (Variables|Default|SetCurrBullets (- (Variables|Default|GetCurrBullets) 1))
          (Development|PrintString "Spawned"))
        (else
          (Variables|Default|SetIsReloading true)
          (Variables|Default|SetReloadDoneTime (+ _returnvalue_2 (Variables|Default|GetReloadTime))))))))