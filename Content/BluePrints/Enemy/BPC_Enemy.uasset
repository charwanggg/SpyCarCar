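; Enemy actor that reacts to AI perception and provides a knockback melee attack.
; Any perception update writes a fixed E_BossState value to the controller's Blackboard "State" key, without checking what was sensed or lost.
; MeleeAttack spawns a BP_HitBox slightly offset toward the given target, passing knockback and itself as attacker and instigator.
; Both events print debug strings.
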(event OnPerceptionUpdated(AIPerception)
  (params (UpdatedActors :type Array%20of%20Actor%20Object%20References))
  (AI|Components|Blackboard|SetValueasEnum (AI|GetBlackboard (Pawn|GetController)) (Utilities|String|StringToName "State") (Utilities|Enum|LiteralenumE_BossState "NewEnumerator0"))
  (Development|PrintString "Sees Player"))

(event EventBeginPlay)

(event Collision|EventActorBeginOverlap
  (params (OtherActor :type Actor%20Object%20Reference)))

(event EventTick
  (params (DeltaSeconds :type Float%20%28single-precision%29)))

(event EventMeleeAttack
  (params (Target :type Actor%20Object%20Reference))
  (bind _self self)
  (bind _returnvalue (Transformation|GetActorTransform _self))
  (bind (_location _rotation _scale) (Math|Transform|BreakTransform _returnvalue))
  (Game|SpawnActorfromClass "/Game/BluePrints/BP_HitBox.BP_HitBox_C" (Math|Transform|MakeTransform (+ _location (* (Math|Vector|Normalize (- (Transformation|GetActorLocation Target) _location)) 5e+01)) _rotation _scale) "Undefined" "MultiplyWithRoot" 0 0.25 2e+02 100 1.2e+03 _self _self)
  (Development|PrintString "Attack"))

(fn ConstructionScript)