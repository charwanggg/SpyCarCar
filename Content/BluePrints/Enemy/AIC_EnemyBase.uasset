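; AIC_EnemyBase is an enemy AI controller that starts the enemy's behavior tree.
; On BeginPlay it runs BT_Enemy, then seeds the blackboard with the player pawn at index 1 and a fixed detection radius.
; Possess and Tick are empty, and the delay and AIMoveTo nodes are unconnected leftovers, so any further logic is left to the tree.
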(event EventBeginPlay
  (bind _returnvalue (AI|GetBlackboard 0))
  (AI|RunBehaviorTree "/Game/BluePrints/Enemy/BT_Enemy.BT_Enemy")
  (AI|Components|Blackboard|SetValueasObject _returnvalue (Variables|Default|GetPlayer%20Key%20Name) (Game|Player|GetPlayerPawn 1))
  (AI|Components|Blackboard|SetValueasFloat _returnvalue (Variables|Default|GetDetection%20Radius%20Key) 1e+03))

(event EventTick
  (params (DeltaSeconds :type Float%20%28single-precision%29)))

(event EventPossess
  (params (PossessedPawn :type Pawn%20Object%20Reference)))

(fn ConstructionScript)