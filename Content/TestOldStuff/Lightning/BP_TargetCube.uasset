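; BP_TargetCube is a moving actor in a lightning test folder, apparently serving as a target.
; On BeginPlay, if MoveInRandomDirection is set, it picks a random horizontal MoveVector, with a wider range on X than on Y.
; Tick moves it by that vector scaled by delta time, teleporting without sweep, so movement ignores blocking collision.
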(event EventBeginPlay
  (if (Variables|Default|GetMoveInRandomDirection)
    (Variables|Default|SetMove%20Vector (Math|Vector|MakeVector (Math|Random|RandomFloatinRange -6e+01 6e+01) (Math|Random|RandomFloatinRange -3e+01 3e+01) 0.0))))

(event Collision|EventActorBeginOverlap
  (params (OtherActor :type Actor%20Object%20Reference)))

(event EventTick
  (params (DeltaSeconds :type Float%20%28single-precision%29))
  (Transformation|SetActorLocation (+ (* (Variables|Default|GetMove%20Vector) DeltaSeconds) (Transformation|GetActorLocation)) false true))

(fn ConstructionScript)