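; BP_LightningConnection is a short-lived effect actor that draws a lightning beam between a start and end actor, with a lightning sphere at the start.
; Tick moves both effects with the actors, collapsing the beam onto the start if the end actor is invalid.
; BeginPlay, after a brief delay, sizes the sphere from the start actor's box or static mesh bounds, plays a pitch-randomized zap, then destroys itself after its lifetime.
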(event EventBeginPlay
  (bind _startactor (Variables|Default|GetStartActor))
  (bind _returnvalue (Actor|GetComponentbyClass _startactor "/Script/Engine.BoxComponent"))
  ;[1 1 1] Set the scale of the lightning sphere
  (Utilities|FlowControl|Delay (stale EventTick DeltaSeconds))
  (Utilities|IsValid _returnvalue
    (:Is%20Valid
      (Niagara|SetNiagaraVariable(Vector3) (Variables|Default|GetLightning%20Sphere) "Sphere Scale" (* (.BoxExtent (Collision|GetComponentBounds _returnvalue)) "0.070000,0.070000,0.070000")))
    (:Is%20Not%20Valid
      (Niagara|SetNiagaraVariable(Vector3) (Variables|Default|GetLightning%20Sphere) "Sphere Scale" (* (.BoxExtent (Collision|GetComponentBounds (Actor|GetComponentbyClass (Variables|Default|GetStartActor) "/Script/Engine.StaticMeshComponent"))) "0.080000,0.080000,0.080000"))))
  (Audio|PlaySoundatLocation "/Game/TestOldStuff/Lightning/simple-zaps-48138.simple-zaps-48138" (Transformation|GetActorLocation (Variables|Default|GetStartActor)) "0, 0, 0" 1.0 (Math|Random|RandomFloatinRange 0.9 1.1) 0.0 0 0 0 0)
  (Utilities|FlowControl|Delay (Variables|Default|GetLifetime))
  (Actor|DestroyActor))

(event EventTick
  (params (DeltaSeconds :type Float%20%28single-precision%29))
  (bind _startactor (Variables|Default|GetStartActor))
  (bind _endactor (Variables|Default|GetEndActor))
  (bind _returnvalue (Transformation|GetActorLocation _startactor))
  ;[1 1 1] Set positions of the lightning connection beam and sphere
  (Niagara|SetNiagaraVariable(Vector3) (Variables|Default|GetLightning%20Sphere) "Origin" _returnvalue)
  (Niagara|SetNiagaraVariable(Vector3) (Variables|Default|GetLightning%20Connection) "Beam start" _returnvalue)
  (Utilities|IsValid _endactor
    (:Is%20Valid
      (Niagara|SetNiagaraVariable(Vector3) (Variables|Default|GetLightning%20Connection) "Beam end" (Transformation|GetActorLocation _endactor)))
    (:Is%20Not%20Valid
      (Niagara|SetNiagaraVariable(Vector3) (Variables|Default|GetLightning%20Connection) "Beam end" _returnvalue))))

(fn ConstructionScript)